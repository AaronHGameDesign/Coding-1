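; BP_CoolBox is an actor that endlessly spawns actors above its Cube once play begins.
; BeginPlay stores a point a fixed height above the Cube and prints it twice on screen for debugging.
; A Delay loop then repeats every SpawnDelay, spawning an actor there at random scale and playing a spatialized PowerUp sound at the box with random pitch.
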(event EventBeginPlay
  (Variables|Default|SetKeySpawnLocation (+ (Transformation|GetWorldLocation (Variables|Default|GetCube)) "0.000000,0.000000,200.000000"))
  (Development|PrintString (Utilities|String|ToString(Vector) (Variables|Default|GetKeySpawnLocation)) true true "(R=0.000000,G=0.660000,B=1.000000,A=1.000000)" 1e+01) ; Just like cout
  (Development|PrintString (Utilities|String|ToString(Vector) (Variables|Default|GetKeySpawnLocation)) true true "(R=1.000000,G=0.296284,B=0.168408,A=1.000000)" 1e+01)
  (Game|SpawnActorfromClass "/Game/Blueprints/BP_Key.BP_Key_C" (Math|Transform|MakeTransform (Variables|Default|GetKeySpawnLocation) "0, 0, 0" (* 1.0 (Math|Random|RandomFloatinRange 0.1 2.0))) "Undefined" "MultiplyWithRoot" 0 0 :!label _label)
  (Audio|SpawnSoundatLocation "/Game/SoundFX/PowerUp.PowerUp" (Transformation|GetWorldLocation (Variables|Default|GetDefaultSceneRoot)) "0, 0, 0" 1.0 (Math|Random|RandomFloatinRange 0.9 1.1) 0.0 "/Game/SoundFX/ATT_Spatial.ATT_Spatial" 0)
  (Utilities|FlowControl|Delay (Variables|Default|GetSpawnDelay))
  (goto _label))

(event Collision|EventActorBeginOverlap
  (params (OtherActor :type Actor%20Object%20Reference)))

(event EventTick
  (params (DeltaSeconds :type Float%20%28single-precision%29)))

(fn ConstructionScript)