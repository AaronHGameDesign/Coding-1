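; Enemy actor that gets a name and team material on BeginPlay and dies when the player character overlaps its capsule.
; An unset name or material is picked by shuffling the matching array and taking the first entry, with debug prints.
; The chosen material is applied to both body and head.
; Player overlap drops Health below zero, and a looping Delay poll, used instead of Tick, then destroys the actor.
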(event OnComponentBeginOverlap(Capsule)
  (params (OverlappedComponent :type Primitive%20Component%20Object%20Reference) (OtherActor :type Actor%20Object%20Reference) (OtherComp :type Primitive%20Component%20Object%20Reference) (OtherBodyIndex :type Integer) (bFromSweep :type Boolean) (SweepResult :type Hit%20Result%20Structure%20%28by%20ref%29))
  (Utilities|Casting|CastToBP_ThirdPersonCharacter OtherActor) ; Did the player hit us
  (Variables|Default|SetHealth -1.0))

(event EventBeginPlay
  (bind _names (Variables|Default|GetNames))
  (bind _materials (Variables|Default|GetMaterials))
  (Utilities|FlowControl|Sequence
    (:then_0
      ;[0.2021 1 0.3424] Every .2 seconds, check to see if health <= 0. If it is, destroy ourselves.
      (Utilities|FlowControl|Delay 0.2 :!label _label)
      (if (<= (Variables|Default|GetHealth) 0.0)
        (Actor|DestroyActor)
        (else
          (goto _label))))
    (:then_1
      (if (== (Variables|Default|GetEnemy%20Names) "") ; If Enemy Name is == to nothing is true Randomize the name. Else, Print the name as it exists.
        (Utilities|Array|Shuffle _names)
        (Variables|Default|SetEnemy%20Names (Utilities|Array|Get(acopy) _names)) ; Set to the randomized name.
      )
      (Development|PrintString (Utilities|String|Append (Utilities|String|ToString(Name) (Variables|Default|GetEnemy%20Names)) "Exists!")))
    (:then_2
      (Utilities|IsValid (Variables|Default|GetEnemy%20Team%20Materials)
        (:Is%20Valid
          (Development|PrintString "A Material Has been set." true true "(R=0.341285,G=1.000000,B=0.378486,A=1.000000)"))
        (:Is%20Not%20Valid
          (Development|PrintString "Let's pick a random material.")
          (Utilities|Array|Shuffle _materials) ; Shuffles the materials, picks first one.
          (Variables|Default|SetEnemy%20Team%20Materials (Utilities|Array|Get(acopy) _materials))))
      (Rendering|Material|SetMaterial (Variables|Default|GetBody) 0 (Variables|Default|GetEnemy%20Team%20Materials)) ; Set the material that was selected.
      (Rendering|Material|SetMaterial (Variables|Default|GetHead) 0 (Variables|Default|GetEnemy%20Team%20Materials)))))

(event Collision|EventActorBeginOverlap
  (params (OtherActor :type Actor%20Object%20Reference)))

(event EventTick
  (params (DeltaSeconds :type Float%20%28single-precision%29)))

(fn ConstructionScript)