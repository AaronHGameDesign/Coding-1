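; BP_Item is an item with a name, an elemental type and damage, which prints debug messages about itself on BeginPlay.
; A Constructor function, called from BeginPlay, picks a name from a hardcoded list when Name is still "Item".
; GetDamage finds the victim's opposite element with modulo-4 wraparound and returns double Damage on a match; BeginPlay tests it against Air.
; An older switch-based element check remains disconnected.
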(event EventBeginPlay
  (CallFunction|Constructor)
  (Development|PrintString (Utilities|String|Append "Hello my name is " (Variables|Default|GetName)))
  (bind _damage (CallFunction|GetDamage "NewEnumerator3"))
  (Development|PrintString (Utilities|String|Append "Our elem type is Earth,victim is air, damage = " (Utilities|String|EnumtoString (Variables|Default|GetElementalType)) ", victim is air, damage = " (Utilities|String|ToString(Integer) _damage)) true true "(R=0.000000,G=0.660000,B=1.000000,A=1.000000)" 5.0))

(event Collision|EventActorBeginOverlap
  (params (OtherActor :type Actor%20Object%20Reference)))

(event EventTick
  (params (DeltaSeconds :type Float%20%28single-precision%29)))

(fn ConstructionScript)

(fn Constructor
  (bind _returnvalue (Utilities|String|MakeLiteralString "John"))
  (bind _returnvalue_2 (Utilities|String|MakeLiteralString "Aaron"))
  (bind _returnvalue_3 (Utilities|String|MakeLiteralString "Jake"))
  (bind _returnvalue_4 (Utilities|String|MakeLiteralString "Ichigo"))
  (bind _array (Utilities|Array|MakeArray _returnvalue_2 _returnvalue_3 _returnvalue_4 _returnvalue))
  (if (Utilities|Enum|Equal(Enum) (Variables|Default|GetName) "Item") ; Randomize if name is not yet set.
    (Utilities|Array|Shuffle _array)
    (Variables|Default|SetName (Utilities|Array|Get(acopy) _array (Math|Random|RandomIntegerinRange (- (Utilities|Array|Length _array) 0) 0)))))

(fn GetDamage
  (params (Victim%20Elem%20Type :type ElementalType%20Enum :default "NewEnumerator1"))
  (LocalVariables|SetReturnDamage (LocalVariables|GetReturnDamage)) ; set returned damage to item;s damage
  (if (== (Class|KismetMathLibrary|PercentByteByte (+ Victim%20Elem%20Type 2) 4) (Math|Conversions|ToInteger(Byte) (Variables|Default|GetElementalType)))
    (LocalVariables|SetReturnDamage (* (Variables|Default|GetDamage) 2)))
  (return (LocalVariables|GetReturnDamage)))